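; BP_EnemyCharacter is an enemy character that flashes when damaged and is destroyed when its BP_HealthComponent signals death.
; The construction script creates a dynamic body material instance set to the original color.
; ProcessDamage only triggers visual feedback, where a timeline lerps the BodyColor parameter between original and hit colors.
; Health changes from the component are printed to screen as debug text.
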(event Die(BP_HealthComponent)
  (Actor|DestroyActor))

(event HealthChanged(BP_HealthComponent)
  (params (Health :type Float%20%28double-precision%29))
  (Development|PrintString (Utilities|String|ToString(Float) Health) true true "(R=1.000000,G=0.324794,B=0.469238,A=1.000000)"))

(event Custom|VisualDamageFeedback
  (bind _colorinterp (Timeline|Material%20Color%20Timeline PlayFromStart)
    (:Update
      (Rendering|Material|SetVectorParameterValue (Variables|Default|GetEnemyMaterial) "BodyColor" (Math|Color|Lerp(LinearColor) (Variables|Default|GetOriginalColor) (Variables|Default|GetHitColor) _colorinterp) :!class /Script/Engine.MaterialInstanceDynamic))))

(event EventBeginPlay
  (|CallParentFunction) ; This node is disabled and will not be called.\nDrag off pins to build functionality.
)

(event Collision|EventActorBeginOverlap
  (params (OtherActor :type Actor%20Object%20Reference))
  (|CallParentFunction OtherActor) ; This node is disabled and will not be called.\nDrag off pins to build functionality.
)

(event EventTick
  (params (DeltaSeconds :type Float%20%28single-precision%29))
  (|CallParentFunction DeltaSeconds) ; This node is disabled and will not be called.\nDrag off pins to build functionality.
)

(fn ConstructionScript
  (|CallParentFunction)
  (bind _returnvalue (Rendering|Material|CreateDynamicMaterialInstance (Variables|Character|GetMesh) 0 "/Game/Plugins/Characters/Mannequin_UE4/Materials/M_MannequinUE4_Body_Inst.M_MannequinUE4_Body_Inst" "None" :!class /Script/Engine.PrimitiveComponent))
  (bind _output_get (Variables|Default|SetEnemyMaterial _returnvalue))
  (Rendering|Material|SetVectorParameterValue _output_get "BodyColor" (Variables|Default|GetOriginalColor) :!class /Script/Engine.MaterialInstanceDynamic))

(fn ProcessDamage
  (CallFunction|VisualDamageFeedback))
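; BP_Weapon is a data-driven weapon actor that configures itself from the DT_Weapon data table.
; On BeginPlay it looks up the row named by WeaponName, stores it as WeaponData, then applies that row's skeletal mesh to WeaponMesh.
; Getters expose WeaponData and WeaponMesh to other code.
; A missing row is silently ignored, and the construction script is empty, so setup happens only at runtime.
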(event EventBeginPlay
  (CallFunction|SetWeaponData)
  (CallFunction|SetWeaponMesh))

(fn ConstructionScript)

(fn SetWeaponData
  (bind _returnvalue (Utilities|GetDataTableRow "/Game/Blueprints/Actors/Weapons/DT_Weapon.DT_Weapon" (Variables|Default|GetWeaponName))
    (:then
      (Variables|Default|SetWeaponData _returnvalue))
    (:RowNotFound
      _))
  (return))

(fn SetWeaponMesh
  (Class|SkinnedMeshComponent|SetSkeletalMesh (Variables|Default|GetWeaponMesh) (.Mesh (Utilities|Struct|BreakFWeaponData (Variables|Default|GetWeaponData))) true)
  (return))

(fn GetWeaponData
  (return (Variables|Default|GetWeaponData)))

(fn GetWeaponMesh
  (return (Variables|Default|GetWeaponMesh)))
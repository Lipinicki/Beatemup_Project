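; Combat component for BP_CombatCharacter that equips weapons and runs light, charged, jump and ranged attacks.
; Inputs select montages from a weapon-type data table by hand, combo counter and airborne state, with a delayed combo reset.
; Melee hits use a looping-timer sphere trace between weapon sockets, sending damage and knockback once per target, stronger for charged or finishing hits.
; It also spawns default or charged projectiles and finds the closest enemy.
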(event Custom|LightAttack
  ;[1 1 1] Proccess melee attacks input
  (if (not (Variables|AttackingState|GetbWasPreviousChargedAttack))
    (Variables|AttackingState|SetbChargeAttack false)
    (else
      (Variables|AttackingState|SetbChargeAttack true)))
  (Utilities|CheckifCanAttack (Variables|Weapons|GetMeleeWeapon)
    (:CanAttack
      (Variables|AttackingState|SetAttackingHand "NewEnumerator0")
      (CallFunction|SetupAttackAnimations))))

(event Custom|ChargedAttack
  ;[1 1 1] Proccess melee attacks input
  (Variables|AttackingState|SetbWasPreviousChargedAttack true)
  (Variables|AttackingState|SetbChargeAttack true)
  (Utilities|CheckifCanAttack (Variables|Weapons|GetMeleeWeapon)
    (:CanAttack
      (Variables|AttackingState|SetAttackingHand "NewEnumerator0")
      (CallFunction|SetupAttackAnimations))))

(event Custom|ShootProjectile
  (if (Variables|AttackingState|GetbChargeAttack)
    (Variables|RangedAttack|SetCurrentProjectileClass (Variables|RangedAttack|GetChargedProjectileClass))
    (else
      (Variables|RangedAttack|SetCurrentProjectileClass (Variables|RangedAttack|GetDefaultProjectileClass))))
  (Game|SpawnActorfromClass (Variables|RangedAttack|GetCurrentProjectileClass) (Variables|Default|GetTarget%20Transform) "Undefined" 0 (Variables|/Script/Engine.Actor|GetInstigator (Variables|Weapons|GetRangedWeapon))))

(event Custom|Shoot
  (params (TargetTransform :type Transform))
  ;[1 1 1] Proccess ranged attacks input (TODO: Light and Charged range attacks)
  (Variables|Default|SetTarget%20Transform TargetTransform)
  (Variables|AttackingState|SetbChargeAttack false)
  (Utilities|CheckifCanAttack (Variables|Weapons|GetRangedWeapon)
    (:CanAttack
      (Variables|AttackingState|SetAttackingHand "NewEnumerator1")
      (CallFunction|SetupAttackAnimations))))

(event Custom|ChargedShoot
  (params (Target%20Transform :type Transform))
  ;[1 1 1] Proccess ranged attacks input (TODO: Light and Charged range attacks)
  (Variables|Default|SetTarget%20Transform Target%20Transform)
  (Variables|AttackingState|SetbChargeAttack true)
  (Utilities|CheckifCanAttack (Variables|Weapons|GetRangedWeapon)
    (:CanAttack
      (Variables|AttackingState|SetAttackingHand "NewEnumerator1")
      (CallFunction|SetupAttackAnimations))))

(event Custom|SetupAttackAnimations
  (bind _combat_character (CallFunction|GetCombatCharacter))
  (bind (_strongattacks _lightattacks _jumpattacks) (CallFunction|GetAttackAnimations))
  (bind _attackanimation (CallFunction|SelectAnimation _jumpattacks))
  (if (Utilities|Enum|NotEqual(Enum) (Variables|/Script/Engine.CharacterMovementComponent|GetMovementMode (Variables|/Script/Engine.Character|GetCharacterMovement (CallFunction|GetCombatCharacter))) "MOVE_Falling")
    (if (Variables|AttackingState|GetbChargeAttack)
      (Animation|PlayAnimMontage _combat_character (CallFunction|SelectAnimation _strongattacks) 1.0 "None")
      (else
        (Animation|PlayAnimMontage _combat_character (CallFunction|SelectAnimation _lightattacks) 1.0 "None")))
    (else
      (Animation|PlayAnimMontage _combat_character _attackanimation 1.0 "None")
      (Utilities|IsValid _attackanimation
        (:Is%20Not%20Valid
          (CallFunction|ResetAttackCounter))))))

(event Custom|ClearAttackCounter
  ;[1 1 1] Give player the ability to follow up with the other attacks of the combo
  (Variables|AttackingState|SetbIsAttacking false)
  (Default|CallOnAttackFinished)
  (Utilities|FlowControl|RetriggerableDelay (Variables|AttackingState|GetClearAttackDelay))
  (Variables|AttackingState|SetAttackCounter 0)
  (Variables|AttackingState|SetbWasPreviousChargedAttack false))

(event Custom|ResetAttackCounter
  ;[1 1 1] Reset attacking state
  (Variables|AttackingState|SetbIsAttacking false)
  (Default|CallOnComboEnded)
  (Variables|AttackingState|SetAttackCounter 0)
  (Variables|AttackingState|SetbWasPreviousChargedAttack false))

(event Custom|TriggerMultiLineTrace
  (bind _returnvalue (Utilities|Time|SetTimerbyEvent (delegate Custom|ApplyMultiLineTrace) 0.03 true))
  (Variables|WeaponTrace|SetMultiLineTraceHandle _returnvalue))

(event Custom|ApplyMultiLineTrace
  (bind _final_damage (CallFunction|GetAttackDamage))
  (bind _attackingweapon (Variables|Weapons|GetAttackingWeapon))
  (bind _weaponmesh (Variables|/Game/Blueprints/Weapons/BP_Weapon.BP_Weapon_C|GetWeaponMesh _attackingweapon))
  (Utilities|FlowControl|Sequence
    (:then_0
      (bind (_outhits _returnvalue) (Collision|MultiSphereTraceByChannel (Transformation|GetSocketLocation _weaponmesh "weapon_base") (Transformation|GetSocketLocation _weaponmesh "weapon_end") (Variables|AttackingState|GetAttackRadius) "TraceTypeQuery1" false (Utilities|Array|MakeArray (Components|GetOwner) (Variables|Weapons|GetMeleeWeapon) (Variables|Weapons|GetRangedWeapon) (Variables|Weapons|GetAttackingWeapon)) "ForDuration" true "(R=1.000000,G=1.000000,B=1.000000,A=1.000000)" "(R=0.000000,G=1.000000,B=0.000000,A=1.000000)" 0.4))
      (if _returnvalue
        (for _array_element _outhits
          (if (Utilities|ClassIsChildOf (Utilities|GetClass (.HitActor (Collision|BreakHitResult _array_element))) (Variables|WeaponTrace|GetCharacterToHit))
            (if (not (Utilities|Array|ContainsItem (Variables|WeaponTrace|GetTargetHits) (.HitActor (Collision|BreakHitResult _array_element))))
              (if (not (Utilities|ClassIsChildOf (Utilities|GetClass (.HitActor (Collision|BreakHitResult _array_element))) (Variables|WeaponTrace|GetClassToIgnore)))
                (Utilities|Array|Add (Variables|WeaponTrace|GetTargetHits) (.HitActor (Collision|BreakHitResult _array_element)))
                (Class|IDamageable|DealDamage(Message) (.HitActor (Collision|BreakHitResult _array_element)) _final_damage)
                (Class|IDamageable|ReceiveKnockback(Message) (.HitActor (Collision|BreakHitResult _array_element)) (Components|GetOwner) (CallFunction|GetKnockbackMultiplier))
                (Development|PrintText (Utilities|Text|FormatText "Damage Taken: {0}" _final_damage) true true "(R=1.000000,G=0.658375,B=0.545725,A=1.000000)")))))))
    (:then_1
      ;[1 1 1] Stops attack trace if is not attacking anymore
      (Utilities|FlowControl|RetriggerableDelay 0.2)
      (if (not (Variables|AttackingState|GetbIsAttacking))
        (CallFunction|StopMultiLineTrace)))))

(event Custom|StopMultiLineTrace
  ;[1 1 1] Called to stop the trace from the attack
  (Utilities|Time|ClearandInvalidateTimerbyHandle (Variables|WeaponTrace|GetMultiLineTraceHandle))
  (Utilities|Array|Clear (Variables|WeaponTrace|GetTargetHits)))

(fn GetCombatCharacter
  (bind _asbp_combat_character (Utilities|Casting|CastToBP_CombatCharacter (Components|GetOwner)))
  (return _asbp_combat_character))

(fn SelectAnimation
  (params (AttacksArray :type Array%20of%20Anim%20Montage%20Object%20References))
  (bind _attackcounter (Variables|AttackingState|GetAttackCounter))
  (if (>= _attackcounter (Utilities|Array|Length AttacksArray))
    (return (Utilities|Array|Get(acopy) AttacksArray (Utilities|Array|LastIndex AttacksArray)))
    (else
      (return (Utilities|Array|Get(acopy) AttacksArray _attackcounter)))))

(fn EquipWeapon
  (params (WeaponName :type Name) (bRightHand :type Boolean))
  (bind _combat_character (CallFunction|GetCombatCharacter))
  (bind _combat_character_2 (CallFunction|GetCombatCharacter))
  (if bRightHand
    ;[1 0.5398 0.05746] Spawn right hand weapon
    (bind _returnvalue (Game|SpawnActorfromClass "/Game/Blueprints/Weapons/BP_Weapon.BP_Weapon_C" (Transformation|GetActorTransform _combat_character_2) "AlwaysSpawn" _combat_character_2 WeaponName 0))
    (bind _output_get (Variables|Weapons|SetMeleeWeapon _returnvalue))
    (Transformation|AttachComponentToComponent (Variables|/Game/Blueprints/Weapons/BP_Weapon.BP_Weapon_C|GetWeaponMesh _output_get) (Variables|/Script/Engine.Character|GetMesh _combat_character_2) (Utilities|Struct|BreakFWeaponData (Default|GetWeaponData _output_get)) "SnapToTarget" "KeepRelative" "KeepWorld" true)
    (else
      ;[1 0.5398 0.05746] Spawn right hand weapon
      (bind _returnvalue_2 (Game|SpawnActorfromClass "/Game/Blueprints/Weapons/BP_Weapon.BP_Weapon_C" (Transformation|GetActorTransform _combat_character) "AlwaysSpawn" _combat_character WeaponName _combat_character))
      (bind _output_get_2 (Variables|Weapons|SetRangedWeapon _returnvalue_2))
      (Transformation|AttachComponentToComponent (Variables|/Game/Blueprints/Weapons/BP_Weapon.BP_Weapon_C|GetWeaponMesh _output_get_2) (Variables|/Script/Engine.Character|GetMesh _combat_character) (Utilities|Struct|BreakFWeaponData (Default|GetWeaponData _output_get_2)) "SnapToTarget" "KeepRelative" "KeepWorld" true)))
  (return))

(fn GetAttackAnimations
  (bind _attackingweapon (Variables|Weapons|GetAttackingWeapon))
  (bind _attackinghand (Variables|AttackingState|GetAttackingHand))
  (bind _weapon_data (Default|GetWeaponData _attackingweapon))
  (bind _type (Utilities|Struct|BreakFWeaponData _weapon_data))
  (bind (_lightattacks _strongattacks _jumpattacks) (CallFunction|GetCorrectAnimations _attackinghand _type))
  (Utilities|IsValid _attackingweapon
    (:Is%20Valid
      (return _strongattacks _lightattacks _jumpattacks))))

(fn GetCorrectAnimations
  (params (EquipedHand :type EEquipedHand%20Enum :default "NewEnumerator0") (WeaponType :type EWeaponTypes%20Enum :default "NewEnumerator0"))
  (bind _returnvalue (Utilities|String|EnumtoString WeaponType))
  (bind _weapontypedatatable (Variables|Weapons|GetWeaponTypeDataTable))
  (bind _returnvalue_2 (Utilities|String|StringToName _returnvalue))
  (switch Utilities|FlowControl|Switch|SwitchonEEquipedHand EquipedHand
    (:NewEnumerator0
      (bind _returnvalue_3 (Utilities|GetDataTableRow _weapontypedatatable _returnvalue_2)
        (:then
          (return (.RightHandLightAttack (Utilities|Struct|BreakFAnimations _returnvalue_3)) (.RightHandStrongAttack (Utilities|Struct|BreakFAnimations _returnvalue_3)) (.RightHandJumpAttack (Utilities|Struct|BreakFAnimations _returnvalue_3))))))
    (:NewEnumerator1
      (bind _returnvalue_4 (Utilities|GetDataTableRow _weapontypedatatable _returnvalue_2)
        (:then
          (return (.LeftHandLightAttack (Utilities|Struct|BreakFAnimations _returnvalue_4)) (.LeftHandStrongAttack (Utilities|Struct|BreakFAnimations _returnvalue_4)) (.LeftHandJumpAttack (Utilities|Struct|BreakFAnimations _returnvalue_4))))))))

(fn IncrementAttackCounter
  (Math|Integer|IncrementInt (Variables|AttackingState|GetAttackCounter)
    (:%20%20
      (return))))

(fn GetAttackDamage
  (bind _attackingweapon (Variables|Weapons|GetAttackingWeapon))
  (bind _weapon_data (Default|GetWeaponData _attackingweapon))
  (bind _damage (Utilities|Struct|BreakFWeaponData _weapon_data))
  (if (CallFunction|IsStrongAttack)
    (return (* _damage (Variables|AttackingState|GetChargedAttackDamageMultiplier)))
    (else
      (return _damage))))

(fn IsStrongAttack
  (return (or (and (Variables|AttackingState|GetbChargeAttack) (== (Variables|AttackingState|GetAttackCounter) 0)) (and (>= (Variables|AttackingState|GetAttackCounter) 2) (not (Variables|AttackingState|GetbWasPreviousChargedAttack))))))

(fn GetKnockbackMultiplier
  (if (CallFunction|IsStrongAttack)
    (return 1.0)
    (else
      (return 0.4))))

(fn SearchforClosestEnemy
  (params (Center%20Actor :type Actor%20Object%20Reference))
  (bind (_outactors _returnvalue) (Collision|SphereOverlapActors (Transformation|GetActorLocation Center%20Actor) (Variables|Default|GetTargetSearchRadius) (Variables|Default|GetObject%20Types) "/Game/Blueprints/Player/BP_CombatCharacter.BP_CombatCharacter_C" (Utilities|Array|MakeArray Center%20Actor (Components|GetOwner) (Variables|Weapons|GetMeleeWeapon) (Variables|Weapons|GetRangedWeapon) (Variables|Weapons|GetAttackingWeapon))))
  (if _returnvalue
    (LocalVariables|SetDistance 4e+62)
    (for _array_element _outactors
      (if (< (Transformation|GetSquaredDistanceTo _array_element Center%20Actor) (LocalVariables|GetDistance))
        (LocalVariables|SetDistance (Transformation|GetSquaredDistanceTo _array_element Center%20Actor))
        (Variables|Default|SetClosestTarget _array_element)))
    (return (Variables|Default|GetClosestTarget))))
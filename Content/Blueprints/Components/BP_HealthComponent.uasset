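; Health component that tracks an actor's current health, handling damage and healing.
; Health starts at the maximum on BeginPlay; ReceiveDamage subtracts damage, clamps at zero and fires the Die event when depleted, returning the new value.
; HealHealth adds a fixed amount capped at the maximum.
; Both functions broadcast HealthChanged with the new health and a flag marking whether it was a hit.
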(event EventBeginPlay
  (Variables|Health|SetCurrentHealth (Variables|Health|GetMaxHealth)))

(fn ReceiveDamage
  (params (Damage :type Float%20%28double-precision%29))
  (if (<= (- (Variables|Health|GetCurrentHealth) Damage) 0.0)
    (Variables|Health|SetCurrentHealth 0.0)
    (Default|CallDie)
    (else
      (Variables|Health|SetCurrentHealth (- (Variables|Health|GetCurrentHealth) Damage))))
  (Default|CallHealthChanged (Variables|Health|GetCurrentHealth) true)
  (return (Variables|Health|GetCurrentHealth)))

(fn HealHealth
  (if (> (+ (Variables|Health|GetCurrentHealth) 15.0) (Variables|Health|GetMaxHealth))
    (bind _output_get (Variables|Health|SetCurrentHealth (Variables|Health|GetMaxHealth)))
    (Default|CallHealthChanged _output_get false)
    (else
      (bind _output_get_2 (Variables|Health|SetCurrentHealth (+ (Variables|Health|GetCurrentHealth) 15.0)))
      (Default|CallHealthChanged _output_get_2 false))))
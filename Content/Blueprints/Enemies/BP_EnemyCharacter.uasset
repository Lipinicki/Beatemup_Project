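; Enemy character that fights with a sword through a combat component, exposing light and charged attack events for AI to call.
; Health changes print the value, set a was-hit Blackboard key for the Behavior Tree and play a hit sound.
; Death destroys attached actors and itself, then fires OnEnemyDeath.
; Construction creates tinted dynamic Manny materials; damage and knockback handlers are empty.
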(event Die(BP_HealthComponent)
  (for _array_element (Actor|GetAttachedActors false true)
    (Actor|DestroyActor _array_element))
  (Actor|DestroyActor)
  (Default|CallOnEnemyDeath))

(event HealthChanged(BP_HealthComponent)
  (params (Health :type Float%20%28double-precision%29))
  (bind _returnvalue (AI|GetBlackboard 0))
  (Development|PrintString (Utilities|String|ToString(Float) Health) true true "(R=1.000000,G=0.324794,B=0.469238,A=1.000000)")
  (Utilities|IsValid _returnvalue
    (:Is%20Valid
      (AI|Components|Blackboard|SetValueasBool _returnvalue (Variables|Default|GetWasHitKeyName) true) ; Notifies Behavior Tree when receiving a hit
      (Audio|PlaySoundatLocation "/Game/SFX/Player/Combat/AC_Player_Hit_02.AC_Player_Hit_02" (Transformation|GetActorLocation) "0, 0, 0" 1.0 1.0 0.0 0 0 0 0))))

(event Custom|AIChargedAttack
  ;[1 1 1] Process AI attack calls
  (Default|ChargedAttack (Variables|Default|GetBP_CombatSystemComponent)))

(event Custom|AIAttack
  ;[1 1 1] Process AI attack calls
  (Default|LightAttack (Variables|Default|GetBP_CombatSystemComponent)))

(event EventBeginPlay
  (|CallParentFunction)
  (Default|EquipWeapon (Variables|Default|GetBP_CombatSystemComponent) "AISword" true))

(event EventProcessKnockback)

(event EventTick
  (params (DeltaSeconds :type Float%20%28single-precision%29))
  (|CallParentFunction DeltaSeconds))

(fn ConstructionScript
  (|CallParentFunction)
  (Utilities|FlowControl|Sequence
    (:then_0
      (bind _returnvalue (Rendering|Material|CreateDynamicMaterialInstance (Variables|Character|GetMesh) 0 "/Game/Plugins/Characters/Mannequins/Materials/Instances/Manny/MI_Manny_02.MI_Manny_02" "None" :!class /Script/Engine.PrimitiveComponent))
      (Utilities|Array|Add (Variables|Default|GetCharacterMaterials) _returnvalue))
    (:then_1
      (bind _returnvalue_2 (Rendering|Material|CreateDynamicMaterialInstance (Variables|Character|GetMesh) 1 "/Game/Plugins/Characters/Mannequins/Materials/Instances/Manny/MI_Manny_01.MI_Manny_01" "None" :!class /Script/Engine.PrimitiveComponent))
      (Utilities|Array|Add (Variables|Default|GetCharacterMaterials) _returnvalue_2))
    (:then_2
      (for _array_element (Variables|Default|GetCharacterMaterials)
        (Rendering|Material|SetVectorParameterValue _array_element "Tint" (Variables|Default|GetOriginalColor) :!class /Script/Engine.MaterialInstanceDynamic)))))

(fn ProcessDamage)
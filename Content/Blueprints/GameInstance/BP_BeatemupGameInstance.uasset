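; BP_BeatemupGameInstance is the beat 'em up's game instance, owning save data, checkpoints and level transitions.
; On Init it loads the default slot or creates a BP_SaveData, and it writes changes back asynchronously.
; Saving a checkpoint records player position, level and reached checkpoints, while per-level lists register unique checkpoints and the start point.
; Changing level wipes checkpoint progress before opening the map; reloading clears only the runtime registry, so saved progress survives.
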(event Custom|NewSave
  (bind _returnvalue (SaveGame|CreateSaveGameObject "/Game/Blueprints/SaveSystem/BP_SaveData.BP_SaveData_C"))
  (Variables|Default|SetCurrentSaveData _returnvalue)
  (CallFunction|SaveGameState))

(event Custom|SaveGameState
  (|AsyncSaveGametoSlot (Variables|Default|GetCurrentSaveData) (Variables|DefaultSaveGameVars|GetDefaultSaveSlotName) (Variables|DefaultSaveGameVars|GetDefault%20User%20Index)))

(event Custom|OpenLastPlayedLevel
  (Game|OpenLevel(byName) (Variables|/Game/Blueprints/SaveSystem/BP_SaveData.BP_SaveData_C|GetLastPlayedLevel (Variables|Default|GetCurrentSaveData))))

(event EventInit
  (bind _returnvalue (SaveGame|DoesSaveGameExist (Variables|DefaultSaveGameVars|GetDefaultSaveSlotName) (Variables|DefaultSaveGameVars|GetDefault%20User%20Index)))
  (if _returnvalue
    (bind _returnvalue_2 (SaveGame|LoadGamefromSlot (Variables|DefaultSaveGameVars|GetDefaultSaveSlotName) (Variables|DefaultSaveGameVars|GetDefault%20User%20Index)))
    (bind _asbp_save_data (Utilities|Casting|CastToBP_SaveData _returnvalue_2))
    (Variables|Default|SetCurrentSaveData _asbp_save_data)
    (else
      (CallFunction|NewSave))))

(fn ValidateCheckpoint
  (params (CheckpointName :type Name) (IsStartOfTheLevel :type Boolean) (CheckpointPos :type Transform))
  (if IsStartOfTheLevel
    (Variables|Default|SetStartCheckpoint CheckpointName)
    (Variables|Default|SetStartCheckpointPos CheckpointPos))
  (bind _returnvalue (Utilities|Array|AddUnique (Variables|Default|GetLevelCheckpoints) CheckpointName))
  (return (>= _returnvalue 0)))

(fn IsStartOftheLevel
  (return (Utilities|Array|IsEmpty (Variables|/Game/Blueprints/SaveSystem/BP_SaveData.BP_SaveData_C|GetReachedCheckpoints (Variables|Default|GetCurrentSaveData)))))

(fn SaveCheckpoint
  (params (CheckpointArea :type BP%20Checkpoint%20Area%20Object%20Reference) (Current%20Level%20Name :type Name))
  (Variables|/Game/Blueprints/SaveSystem/BP_SaveData.BP_SaveData_C|SetLastPlayerPos (Variables|Default|GetCurrentSaveData) (Default|GetActualSavePosition CheckpointArea))
  (Variables|/Game/Blueprints/SaveSystem/BP_SaveData.BP_SaveData_C|SetLastPlayedLevel (Variables|Default|GetCurrentSaveData) Current%20Level%20Name)
  (bind _success (Default|SaveCheckpoint (Variables|Default|GetCurrentSaveData) (Utilities|String|ToString(Name) (Variables|/Game/Blueprints/LevelDesign/BP_CheckpointArea.BP_CheckpointArea_C|GetCheckpointName CheckpointArea))))
  (CallFunction|SaveGameState)
  (return _success))

(fn IsCheckpointSaved
  (params (Checkpoint%20Name :type String))
  (return (Utilities|Array|ContainsItem (Variables|/Game/Blueprints/SaveSystem/BP_SaveData.BP_SaveData_C|GetReachedCheckpoints (Variables|Default|GetCurrentSaveData)) Checkpoint%20Name)))

(fn ChangeLevel
  (params (LevelName :type Name))
  (bind _currentsavedata (Variables|Default|GetCurrentSaveData))
  (CallFunction|ClearInstanceData)
  (Variables|Default|SetStartCheckpointPos "")
  (Variables|/Game/Blueprints/SaveSystem/BP_SaveData.BP_SaveData_C|SetLastPlayerPos _currentsavedata "")
  (Utilities|Array|Clear (Variables|/Game/Blueprints/SaveSystem/BP_SaveData.BP_SaveData_C|GetReachedCheckpoints _currentsavedata))
  (Variables|/Game/Blueprints/SaveSystem/BP_SaveData.BP_SaveData_C|SetLastPlayedLevel (Variables|Default|GetCurrentSaveData) LevelName)
  (CallFunction|SaveGameState)
  (Game|OpenLevel(byName) LevelName))

(fn ClearInstanceData
  (Utilities|Array|Clear (Variables|Default|GetLevelCheckpoints))
  (Variables|Default|SetStartCheckpoint "None"))

(fn ReloadLevelfromCheckpoint
  (CallFunction|ClearInstanceData)
  (bind _returnvalue (Game|GetCurrentLevelName true))
  (Game|OpenLevel(byName) (Utilities|String|StringToName _returnvalue)))
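; Beat 'em up game mode that handles checkpoint spawning, death restarts and Articy-driven dialogue.
; BeginPlay seeds the save with the start checkpoint if none is reached, moves the player to the saved position and creates the dialogue HUD.
; Player death reloads the saved level after a short delay.
; Articy flow player events fill speaker, text and branch or close buttons, while PlayDialogue and EndDialogue toggle widget visibility and input mode.
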(event OnPlayerPaused(ArticyFlowPlayer)
  (params (PausedOn :type Articy%20Flow%20Object%20Interface))
  (bind _playerhud (Variables|Default|GetPlayerHUD))
  (bind _playerhud_2 (Variables|Default|GetPlayerHUD))
  (bind _asarticy_node (Utilities|Casting|CastToArticyNode PausedOn))
  (switch Utilities|FlowControl|Switch|SwitchonEArticyPausableType (Class|ArticyNode|GetType _asarticy_node)
    (:Dialogue
      (Class|ArticyFlowPlayer|Play (Variables|Default|GetArticyFlowPlayer)))
    (:DialogueFragment
      (Utilities|FlowControl|Sequence
        (:then_0
          (bind _asarticy_object_with_text (Utilities|Casting|CastToArticyObjectWithText PausedOn))
          (bind _returnvalue (Class|ArticyObjectwithText|GetText _asarticy_object_with_text))
          (Utilities|IsValid _playerhud_2
            (:Is%20Valid
              (Rendering|Components|TextRender|SetText (Variables|/Game/Developers/Mondini/Collections/02-Narrative/WBP_Dialogue.WBP_Dialogue_C|GetDialogueText (Variables|/Game/Developers/Mondini/Collections/02-Narrative/WBP_DialogueHUD.WBP_DialogueHUD_C|GetDialogueWidget _playerhud_2)) _returnvalue))))
        (:then_1
          (bind _asarticy_object_with_speaker (Utilities|Casting|CastToArticyObjectWithSpeaker PausedOn))
          (bind _returnvalue_2 (Class|ArticyObjectwithDisplayName|GetDisplayName(Message) (Class|ArticyObjectwithSpeaker|GetSpeaker _asarticy_object_with_speaker)))
          (Utilities|IsValid _playerhud
            (:Is%20Valid
              (Rendering|Components|TextRender|SetText (Variables|/Game/Developers/Mondini/Collections/02-Narrative/WBP_Dialogue.WBP_Dialogue_C|GetSpeakerName (Variables|/Game/Developers/Mondini/Collections/02-Narrative/WBP_DialogueHUD.WBP_DialogueHUD_C|GetDialogueWidget _playerhud)) _returnvalue_2))))))))

(event OnBranchesUpdated(ArticyFlowPlayer)
  (params (AvailableBranches :type Array%20of%20Articy%20Branch%20Structures))
  (Utilities|FlowControl|Sequence
    (:then_0
      (Widget|Panel|ClearChildren (Variables|Default|GetWrap%20Box%20Branches)))
    (:then_1
      (for _array_element AvailableBranches
        (Utilities|Casting|CastToKitty_Ao_Resgate_draft_DialogueFragment (Class|ArticyFunctionLibrary|GetBranchTarget _array_element))
        (bind _returnvalue (UserInterface|CreateWidget "/Game/Developers/Mondini/Collections/02-Narrative/WBP_BranchButton.WBP_BranchButton_C"))
        (Widget|Panel|AddChild (Variables|Default|GetWrap%20Box%20Branches) _returnvalue)
        (Default|AssignBranch _returnvalue (Variables|Default|GetArticyFlowPlayer) _array_element)))
    (:then_2
      (if (not (Class|PanelWidget|HasAnyChildren (Variables|Default|GetWrap%20Box%20Branches)))
        (bind _returnvalue_2 (UserInterface|CreateWidget "/Game/Developers/Mondini/Collections/02-Narrative/WBP_CloseButton.WBP_CloseButton_C"))
        (Widget|Panel|AddChild (Variables|Default|GetWrap%20Box%20Branches) _returnvalue_2)))))

(event Custom|PlayerDeath
  (Utilities|FlowControl|RetriggerableDelay 2.3)
  (Game|OpenLevel(byName) (Variables|/Game/Blueprints/SaveSystem/BP_SaveData.BP_SaveData_C|GetCurrentLevel (Variables|/Game/Blueprints/LevelDesign/BP_BeatemupGameInstance.BP_BeatemupGameInstance_C|GetCurrentSaveData (.AsBP%20Beatemup%20Game%20Instance (Utilities|Casting|CastToBP_BeatemupGameInstance (Game|GetGameInstance)))))))

(event Custom|SpawnPlayer
  (Transformation|SetActorLocation (Variables|Default|GetPlayer%20Beatemup%20Character) (.Location (Math|Transform|BreakTransform (Variables|/Game/Blueprints/SaveSystem/BP_SaveData.BP_SaveData_C|GetLastPlayerPos (Variables|/Game/Blueprints/LevelDesign/BP_BeatemupGameInstance.BP_BeatemupGameInstance_C|GetCurrentSaveData (.AsBP%20Beatemup%20Game%20Instance (Utilities|Casting|CastToBP_BeatemupGameInstance (Game|GetGameInstance))))))) false false))

(event EventBeginPlay
  (bind _returnvalue (Game|GetGameInstance))
  (bind _returnvalue_2 (Game|GetGameInstance))
  (bind _asbp_beatemup_game_instance (Utilities|Casting|CastToBP_BeatemupGameInstance _returnvalue_2))
  (bind _asbp_beatemup_game_instance_2 (Utilities|Casting|CastToBP_BeatemupGameInstance _returnvalue))
  (bind _currentsavedata (Variables|/Game/Blueprints/LevelDesign/BP_BeatemupGameInstance.BP_BeatemupGameInstance_C|GetCurrentSaveData _asbp_beatemup_game_instance))
  (bind _currentsavedata_2 (Variables|/Game/Blueprints/LevelDesign/BP_BeatemupGameInstance.BP_BeatemupGameInstance_C|GetCurrentSaveData _asbp_beatemup_game_instance_2))
  (bind _asbp_beatemup_character (Utilities|Casting|CastToBP_BeatemupCharacter (Game|GetPlayerCharacter 0)))
  (bind _output_get (Variables|Default|SetPlayer%20Beatemup%20Character _asbp_beatemup_character))
  (EventDispatchers|BindEventtoOnDeath _output_get (delegate Custom|PlayerDeath))
  (Variables|/Script/Engine.SpringArmComponent|SetbEnableCameraLag (Variables|/Game/Blueprints/Player/BP_BeatemupCharacter.BP_BeatemupCharacter_C|GetCameraBoom (Variables|Default|GetPlayer%20Beatemup%20Character)) false)
  (bind _returnvalue_3 (Game|GetCurrentLevelName true))
  (if (and (not (Default|ContainsCheckpoint _currentsavedata_2 _returnvalue_3 (Utilities|String|ToString(Name) (Variables|/Game/Blueprints/LevelDesign/BP_BeatemupGameInstance.BP_BeatemupGameInstance_C|GetStartCheckpoint _asbp_beatemup_game_instance_2)))) (Utilities|Array|IsEmpty (Variables|/Game/Blueprints/SaveSystem/BP_SaveData.BP_SaveData_C|GetReachedCheckpoints _currentsavedata_2)))
    (Variables|/Game/Blueprints/SaveSystem/BP_SaveData.BP_SaveData_C|SetLastPlayerPos _currentsavedata (Variables|/Game/Blueprints/LevelDesign/BP_BeatemupGameInstance.BP_BeatemupGameInstance_C|GetStartCheckpointPos _asbp_beatemup_game_instance))
    (bind _returnvalue_4 (Game|GetCurrentLevelName true))
    (bind _output_get_2 (Variables|/Game/Blueprints/SaveSystem/BP_SaveData.BP_SaveData_C|SetCurrentLevel _currentsavedata (Utilities|String|StringToName _returnvalue_4)))
    (Default|SaveCheckpoint _currentsavedata (Utilities|String|ToString(Name) _output_get_2) (Utilities|String|ToString(Name) (Variables|/Game/Blueprints/LevelDesign/BP_BeatemupGameInstance.BP_BeatemupGameInstance_C|GetStartCheckpoint _asbp_beatemup_game_instance)))
    (Default|SaveGameState _asbp_beatemup_game_instance))
  (CallFunction|SpawnPlayer)
  (Utilities|FlowControl|Sequence
    (:then_0
      ;[0.67 1 0.6944] Narrative Widget
      (bind _returnvalue_5 (UserInterface|CreateWidget "/Game/Developers/Mondini/Collections/02-Narrative/WBP_DialogueHUD.WBP_DialogueHUD_C" (Game|GetPlayerController 0)))
      (bind _output_get_3 (Variables|Default|SetPlayerHUD _returnvalue_5))
      (UserInterface|Viewport|AddtoViewport _output_get_3 0)
      (Widget|SetVisibility _output_get_3 "Hidden"))
    (:then_1
      (Variables|Default|SetWrap%20Box%20Branches (Variables|/Game/Developers/Mondini/Collections/02-Narrative/WBP_Dialogue.WBP_Dialogue_C|GetWrapBox_Branches (Variables|/Game/Developers/Mondini/Collections/02-Narrative/WBP_DialogueHUD.WBP_DialogueHUD_C|GetDialogueWidget (Variables|Default|GetPlayerHUD)))))))

(event EventTick
  (params (DeltaSeconds :type Float%20%28single-precision%29)))

(fn ConstructionScript)

(fn EndDialogue
  (Widget|SetVisibility (Variables|/Game/Developers/Mondini/Collections/02-Narrative/WBP_DialogueHUD.WBP_DialogueHUD_C|GetDialogueWidget (Variables|Default|GetPlayerHUD)) "Hidden")
  (Input|SetInputModeGameOnly (Game|GetPlayerController 0))
  (Variables|/Game/Developers/Mondini/Collections/02-Narrative/WBP_DialogueHUD.WBP_DialogueHUD_C|SetIsPlayingDialogue (Variables|Default|GetPlayerHUD) false)
  (Class|ArticyFlowPlayer|FinishCurrentPausedObject (Variables|Default|GetArticyFlowPlayer)))

(fn PlayDialogue
  (params (Articy%20Ref :type Articy%20Ref%20Structure))
  (Input|SetInputModeUIOnly (Game|GetPlayerController 0) 0 "DoNotLock")
  (Widget|SetVisibility (Variables|/Game/Developers/Mondini/Collections/02-Narrative/WBP_DialogueHUD.WBP_DialogueHUD_C|GetDialogueWidget (Variables|Default|GetPlayerHUD)) "Visible")
  (Variables|/Game/Developers/Mondini/Collections/02-Narrative/WBP_DialogueHUD.WBP_DialogueHUD_C|SetIsPlayingDialogue (Variables|Default|GetPlayerHUD) true)
  (Class|ArticyFlowPlayer|SetStartNode (Variables|Default|GetArticyFlowPlayer) Articy%20Ref))
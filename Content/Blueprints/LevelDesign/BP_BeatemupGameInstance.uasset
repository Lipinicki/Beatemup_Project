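; Game instance for the beat 'em up that owns the current save data and a registry of checkpoints.
; On Init it loads the default save slot and prints its reached checkpoints for debugging, or creates a new save if none exists.
; Save events write to that slot asynchronously.
; TryAddCheckpoint registers unique checkpoint names, records the level's start checkpoint and position, and returns whether the name was newly added.
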(event Custom|NewSave
  (bind _returnvalue (SaveGame|CreateSaveGameObject "/Game/Blueprints/SaveSystem/BP_SaveData.BP_SaveData_C"))
  (bind _output_get (Variables|Default|SetCurrentSaveData _returnvalue))
  (|AsyncSaveGametoSlot _output_get (Variables|DefaultSaveGameVars|GetDefaultSaveSlotName) (Variables|DefaultSaveGameVars|GetDefault%20User%20Index)))

(event Custom|SaveGameState
  (|AsyncSaveGametoSlot (Variables|Default|GetCurrentSaveData) (Variables|DefaultSaveGameVars|GetDefaultSaveSlotName) (Variables|DefaultSaveGameVars|GetDefault%20User%20Index)))

(event EventInit
  (bind _returnvalue (SaveGame|DoesSaveGameExist (Variables|DefaultSaveGameVars|GetDefaultSaveSlotName) (Variables|DefaultSaveGameVars|GetDefault%20User%20Index)))
  (if _returnvalue
    (bind _returnvalue_2 (SaveGame|LoadGamefromSlot (Variables|DefaultSaveGameVars|GetDefaultSaveSlotName) (Variables|DefaultSaveGameVars|GetDefault%20User%20Index)))
    (bind _asbp_save_data (Utilities|Casting|CastToBP_SaveData _returnvalue_2))
    (bind _output_get (Variables|Default|SetCurrentSaveData _asbp_save_data))
    (Development|PrintString (Utilities|String|JoinStringArray (Variables|/Game/Blueprints/SaveSystem/BP_SaveData.BP_SaveData_C|GetReachedCheckpoints _output_get) ";\\n"))
    (else
      (CallFunction|NewSave))))

(fn TryAddCheckpoint
  (params (CheckpointName :type Name) (IsStartOfTheLevel :type Boolean) (CheckpointPos :type Transform))
  (if IsStartOfTheLevel
    (Variables|Default|SetStartCheckpoint CheckpointName)
    (Variables|Default|SetStartCheckpointPos CheckpointPos))
  (bind _returnvalue (Utilities|Array|AddUnique (Variables|Default|GetGameCheckpoints) CheckpointName))
  (return (>= _returnvalue 0)))
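; BP_CombatArea is a beat 'em up encounter arena that locks the player in until all spawned enemies die.
; Player overlap with the trigger spawns enemies at actor-relative offsets, enables both barriers and fades in their dynamic lock materials via timeline.
; Enemy death events decrement a counter; at zero, the exit opens and locks fade out.
; Flags optionally reopen the entrance and load a target level through the game instance.
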(event OnComponentBeginOverlap(StartCombatTrigger)
  (params (OverlappedComponent :type Primitive%20Component%20Object%20Reference) (OtherActor :type Actor%20Object%20Reference) (OtherComp :type Primitive%20Component%20Object%20Reference) (OtherBodyIndex :type Integer) (bFromSweep :type Boolean) (SweepResult :type Hit%20Result%20Structure%20%28by%20ref%29))
  (Utilities|Casting|CastToBP_BeatemupCharacter OtherActor)
  (for _array_element (Variables|Default|GetEnemiesToSpawn)
    (bind _returnvalue (Game|SpawnActorfromClass (.EnemyType (Utilities|Struct|BreakFSpawnArguments _array_element)) (Math|Transform|MakeTransform (+ (.Location (Math|Transform|BreakTransform (.SpawnLocation (Utilities|Struct|BreakFSpawnArguments _array_element)))) (Transformation|GetActorLocation))) "Undefined" self "(R=1.000000,G=0.000000,B=0.000000,A=0.000000)" 3e+02 0))
    (EventDispatchers|BindEventtoOnEnemyDeath _returnvalue (delegate Custom|EnemyDied))
    (Math|Integer|IncrementInt (Variables|Default|GetRemainingEnemies)))
  (CallFunction|StartCombat))

(event Custom|EnemyDied
  (bind _result (Math|Integer|DecrementInt (Variables|Default|GetRemainingEnemies))
    (:%20%20
      (if (<= _result 0)
        (CallFunction|EndCombat)))))

(event Custom|EndCombat
  (Collision|SetCollisionEnabled (Variables|Default|GetExitCollision) "NoCollision")
  (bind _alphatrack (Timeline|FadeOutLock Play)
    (:Update
      (Rendering|Material|SetScalarParameterValue (Variables|Default|GetExitLockMaterial) "Alpha" _alphatrack :!class /Script/Engine.MaterialInstanceDynamic)
      (if (Variables|Default|GetShouldLetEntranceOpen)
        (Rendering|Material|SetScalarParameterValue (Variables|Default|GetEntranceLockMaterial) "Alpha" _alphatrack :!class /Script/Engine.MaterialInstanceDynamic)))
    (:Finished
      (if (Variables|Default|GetShouldLetEntranceOpen)
        (Collision|SetCollisionEnabled (Variables|Default|GetEntranceCollision) "NoCollision"))
      (if (Variables|Default|GetLoad%20Level%20On%20Combat%20End)
        (Default|ChangeLevel (.AsBP%20Beatemup%20Game%20Instance (Utilities|Casting|CastToBP_BeatemupGameInstance (Game|GetGameInstance))) (Variables|Default|GetTarget%20Level%20To%20Load))))))

(event Custom|StartCombat
  (Collision|SetCollisionEnabled (Variables|Default|GetEntranceCollision) "QueryAndPhysics")
  (Collision|SetCollisionEnabled (Variables|Default|GetExitCollision) "QueryAndPhysics")
  (Collision|SetCollisionEnabled (Variables|Default|GetStartCombatTrigger) "NoCollision")
  (bind _alphatrack (Timeline|FadeInLock Play)
    (:Update
      (Rendering|Material|SetScalarParameterValue (Variables|Default|GetExitLockMaterial) "Alpha" _alphatrack :!class /Script/Engine.MaterialInstanceDynamic)
      (Rendering|Material|SetScalarParameterValue (Variables|Default|GetEntranceLockMaterial) "Alpha" _alphatrack :!class /Script/Engine.MaterialInstanceDynamic))))

(event EventBeginPlay
  (Collision|SetCollisionEnabled (Variables|Default|GetEntranceCollision) "NoCollision")
  (Collision|SetCollisionEnabled (Variables|Default|GetExitCollision) "QueryAndPhysics")
  (Rendering|Material|SetScalarParameterValue (Variables|Default|GetExitLockMaterial) "Alpha" 0.0 :!class /Script/Engine.MaterialInstanceDynamic)
  (Rendering|Material|SetScalarParameterValue (Variables|Default|GetEntranceLockMaterial) "Alpha" 0.0 :!class /Script/Engine.MaterialInstanceDynamic))

(fn ConstructionScript
  (bind _returnvalue (Rendering|Material|CreateDynamicMaterialInstance (Variables|Default|GetEntranceLock) 0 "/Game/Art/MI_Locked.MI_Locked" "None" :!class /Script/Engine.PrimitiveComponent))
  (Variables|Default|SetEntranceLockMaterial _returnvalue)
  (bind _returnvalue_2 (Rendering|Material|CreateDynamicMaterialInstance (Variables|Default|GetExitLock) 0 "/Game/Art/MI_Locked.MI_Locked" "None" :!class /Script/Engine.PrimitiveComponent))
  (Variables|Default|SetExitLockMaterial _returnvalue_2))
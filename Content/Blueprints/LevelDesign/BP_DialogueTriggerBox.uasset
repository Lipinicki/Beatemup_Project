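; BP_DialogueTriggerBox is a level-design trigger volume that plays dialogue when a beat-em-up character is inside it.
; On BeginPlay it checks for characters already overlapping its collision component, and afterwards it reacts to each new begin overlap from a BP_BeatemupCharacter.
; Both paths pass its DialogueReference to PlayDialogue on BP_BeatemupGameMode, with no guard against repeat triggering.
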(event OnComponentBeginOverlap(CollisionComponent)
  (params (OverlappedComponent :type Primitive%20Component%20Object%20Reference) (OtherActor :type Actor%20Object%20Reference) (OtherComp :type Primitive%20Component%20Object%20Reference) (OtherBodyIndex :type Integer) (bFromSweep :type Boolean) (SweepResult :type Hit%20Result%20Structure%20%28by%20ref%29))
  (Utilities|Casting|CastToBP_BeatemupCharacter OtherActor)
  (bind _asbp_beatemup_game_mode (Utilities|Casting|CastToBP_BeatemupGameMode (Game|GetGameMode)))
  (Default|PlayDialogue _asbp_beatemup_game_mode (Variables|Default|GetDialogueReference)))

(event EventBeginPlay
  (if (Utilities|Array|IsNotEmpty (Collision|GetOverlappingActors (Variables|Default|GetCollisionComponent) "/Game/Blueprints/Player/BP_BeatemupCharacter.BP_BeatemupCharacter_C" :!class /Script/Engine.PrimitiveComponent))
    (bind _asbp_beatemup_game_mode (Utilities|Casting|CastToBP_BeatemupGameMode (Game|GetGameMode)))
    (Default|PlayDialogue _asbp_beatemup_game_mode (Variables|Default|GetDialogueReference))))

(fn ConstructionScript)
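; Combat character Blueprint, apparently a base class, that handles taking damage and being knocked back.
; DealDamage forwards damage to the health component, calls the empty ProcessDamage hook, then plays a timeline that lerps character material colors between original and hit colors.
; Knockback stops movement and launches the character away from the source, with horizontal push scaled by multiplier and intensity, plus upward lift scaled by intensity alone.
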(event EventBeginPlay)

(event Collision|EventActorBeginOverlap
  (params (OtherActor :type Actor%20Object%20Reference)))

(event EventTick
  (params (DeltaSeconds :type Float%20%28single-precision%29)))

(event EventDealDamage
  (params (Damage :type Float%20%28double-precision%29))
  (Default|ReceiveDamage (Variables|Default|GetBP_HealthComponent) Damage)
  (CallFunction|ProcessDamage)
  (Utilities|IsValid self
    (:Is%20Valid
      (bind _colorinterp (Timeline|Timeline_0 PlayFromStart)
        (:Update
          (for _array_element (Variables|Default|GetCharacterMaterials)
            (Rendering|Material|SetVectorParameterValue _array_element (Variables|Default|GetColorParamName) (Math|Color|Lerp(LinearColor) (Variables|Default|GetOriginalColor) (Variables|Default|GetHitColor) _colorinterp) :!class /Script/Engine.MaterialInstanceDynamic)))))))

(event EventKnockback
  (params (Source :type Actor%20Object%20Reference) (KnockbackMultiplier :type Float%20%28double-precision%29))
  (bind _returnvalue (Transformation|GetActorLocation))
  (bind _returnvalue_2 (Transformation|GetActorLocation Source))
  (bind _returnvalue_3 (Math|Vector|GetUnitDirection(Vector) _returnvalue_2 _returnvalue))
  (Class|NavMovementComponent|StopActiveMovement (Variables|Character|GetCharacterMovement))
  (Character|LaunchCharacter (* (Math|Vector|MakeVector (* KnockbackMultiplier (.x _returnvalue_3)) (* KnockbackMultiplier (.y _returnvalue_3)) 0.2) (Variables|Default|GetKnockbackIntensity)) true true))

(fn ConstructionScript)

(fn ProcessDamage)
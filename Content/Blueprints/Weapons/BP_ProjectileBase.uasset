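; Base projectile actor that deals damage to the first actor it overlaps other than its Instigator.
; On overlap it sends a DealDamage message carrying its Damage value to that actor, then destroys itself.
; A trailing debug step casts the hit actor to BP_CombatCharacter and prints its current health from the health component.
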(event EventBeginPlay)

(event Collision|EventActorBeginOverlap
  (params (OtherActor :type Actor%20Object%20Reference))
  (if (!= OtherActor (Variables|Actor|GetInstigator))
    (Class|IDamageable|DealDamage(Message) OtherActor (Variables|Default|GetDamage))
    (Actor|DestroyActor)
    ;[1 1 1] Debugging
    (bind _asbp_combat_character (Utilities|Casting|CastToBP_CombatCharacter OtherActor))
    (Utilities|IsValid _asbp_combat_character
      (:Is%20Valid
        (Development|PrintText (Utilities|Text|FormatText "{0} health: {1}" _asbp_combat_character (Variables|/Game/Blueprints/Components/BP_HealthComponent.BP_HealthComponent_C|GetCurrentHealth (Variables|/Game/Blueprints/Player/BP_CombatCharacter.BP_CombatCharacter_C|GetBP_HealthComponent _asbp_combat_character))))))))

(fn ConstructionScript)